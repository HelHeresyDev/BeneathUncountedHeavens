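; BP_Fighter is the fighter actor for the TacticalDuel prototype, representing a player or opponent unit, or a ghost version of one.
; The construction script picks the body material from the IsGhost flag and Team value, with team 0 using the player look and others the opponent look.
; BeginPlay sets the body mesh to a cylinder, and ApplyMaterial allows the material to be overridden.
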(event `self.ReceiveBeginPlay`
  (`StaticMeshComponent.SetStaticMesh` (`self.BodyMesh`) "/Engine/BasicShapes/Cylinder.Cylinder"))

(fn `ApplyMaterial`
  (params (Material :type "MaterialInterface Object Reference"))
  (`PrimitiveComponent.SetMaterial` (`self.BodyMesh`) 0 Material))

(fn `UserConstructionScript`
  (bind _bodymesh (`self.BodyMesh`))
  (if (`self.bIsGhost`)
    (if (== (`self.Team`) 0)
      (`PrimitiveComponent.SetMaterial` _bodymesh 0 "/Game/BUH/Prototypes/TacticalDuel/Materials/MI_GhostPlayer.MI_GhostPlayer")
      (else
        (`PrimitiveComponent.SetMaterial` _bodymesh 0 "/Game/BUH/Prototypes/TacticalDuel/Materials/MI_GhostOpponent.MI_GhostOpponent")))
    (elif (== (`self.Team`) 0)
      (`PrimitiveComponent.SetMaterial` _bodymesh 0 "/Game/BUH/Prototypes/TacticalDuel/Materials/MI_Player.MI_Player")
      (else
        (`PrimitiveComponent.SetMaterial` _bodymesh 0 "/Game/BUH/Prototypes/TacticalDuel/Materials/MI_Opponent.MI_Opponent")))))